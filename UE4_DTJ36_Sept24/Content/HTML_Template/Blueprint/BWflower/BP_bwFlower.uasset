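; Flower actor that drives an ever-expanding spherical mask through the MPC_bwFlower material parameter collection, with a configurable flower mesh.
; From BeginPlay, a looping timer grows the Sphere component radius by one unit about 30 times a second.
; Each step writes actor location and radius to collection parameters named by prefix plus MaskInt, giving indexed mask slots.
; The construction script applies the initial radius, mask values and mesh.
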(event Custom|E_UpdateMask
  (bind _returnvalue (Transformation|GetActorLocation))
  (Rendering|Material|SetVectorParameterValue "/Game/HTML_Template/Blueprint/BWflower/MPC_bwFlower.MPC_bwFlower" (Utilities|String|StringToName (Utilities|String|Append (Variables|Default|GetLocName) (Utilities|String|ToString(Integer) (Variables|Default|GetMaskInt)))) (Utilities|Struct|MakeLinearColor (.x _returnvalue) (.y _returnvalue) (.z _returnvalue) 1.0) :!class /Script/Engine.KismetMaterialLibrary)
  (Rendering|Material|SetScalarParameterValue "/Game/HTML_Template/Blueprint/BWflower/MPC_bwFlower.MPC_bwFlower" (Utilities|String|StringToName (Utilities|String|Append (Variables|Default|GetRadName) (Utilities|String|ToString(Integer) (Variables|Default|GetMaskInt)))) (Variables|Default|GetSphereRadius) :!class /Script/Engine.KismetMaterialLibrary))

(event Custom|E_StartMaskTimer
  (Utilities|Time|SetTimerbyEvent (delegate Custom|E_MaskExpansion) 0.033333 true))

(event Custom|E_MaskExpansion
  (bind _sphere (Variables|Default|GetSphere))
  (bind _output_get (Variables|Default|SetSphereRadius (+ (Variables|/Script/Engine.SphereComponent|GetSphereRadius _sphere) 1.0)))
  (Components|Sphere|SetSphereRadius _sphere _output_get true)
  (CallFunction|EUpdateMask))

(event EventBeginPlay
  (CallFunction|EStartMaskTimer))

(fn ConstructionScript
  (bind _flowermesh (Variables|Default|GetFlowerMesh))
  (Components|Sphere|SetSphereRadius (Variables|Default|GetSphere) (Variables|Default|GetSphereRadius) true)
  (CallFunction|EUpdateMask)
  (Components|StaticMesh|SetStaticMesh _flowermesh (Variables|Default|GetSM_FlowerMesh))
  (Rendering|Material|SetMaterial _flowermesh 0 0))