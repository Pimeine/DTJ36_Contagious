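; Game mode for the HTML game template that runs the flow from main menu to play and manages the UI.
; BeginPlay shows the main menu over a menu camera view, and further events handle pause, the FPS panel and loading screens.
; Starting the game shows a data-table loading image, blocking-loads the starting stream levels, then spawns the player.
; Spawning breaks at the first valid BP_PlayerStart and starts mask timers on BP_bwFlower actors.
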(event Custom|E_AddFpsPanel
  (params (IsVisible :type Boolean))
  ;[0 0 0] Create FPS Panel from Option Panel
  (if IsVisible
    (Variables|Default|GetWBP_FpsPanel
      (:then)
      (:else
        (bind _returnvalue (UserInterface|CreateWidget "/Game/HTML_Template/Blueprint/Widget/Panels/WBP_FpsPanel.WBP_FpsPanel_C" (Game|GetPlayerController 0)))
        (bind _output_get (Variables|Default|SetWBP_FpsPanel _returnvalue))
        (UserInterface|Viewport|AddtoViewport _output_get 0)))
    (else
      (bind _wbp_fpspanel (Variables|Default|GetWBP_FpsPanel)
        (:then
          (Widget|RemovefromParent _wbp_fpspanel)
          (Variables|Default|SetWBP_FpsPanel 0))
        (:else)))))

(event Custom|E_PauseGame
  (params (IsPaused :type Boolean))
  (bind _returnvalue (Game|GetPlayerController 0))
  ;[0 0 0] Create Pause Menu and manage Display On Paused
  (if IsPaused
    (Game|SetGamePaused true)
    (bind _wbp_pausemenu (Variables|Default|GetWBP_PauseMenu)
      (:then
        (UserInterface|Viewport|AddtoViewport _wbp_pausemenu 0))
      (:else
        (bind _returnvalue_2 (UserInterface|CreateWidget "/Game/HTML_Template/Blueprint/Widget/WBP_PausedGame.WBP_PausedGame_C" (Game|GetPlayerController 0)))
        (bind _output_get (Variables|Default|SetWBP_PauseMenu _returnvalue_2))
        (UserInterface|Viewport|AddtoViewport _output_get 0)
        (EventDispatchers|BindEventtoResumeGame _output_get (EventDispatchers|CreateEvent :!event Custom|BE_ResumeGame))))
    (else
      (Game|SetGamePaused false)
      (bind _wbp_pausemenu_2 (Variables|Default|GetWBP_PauseMenu)
        (:then
          (Utilities|IsValid (Variables|/Game/HTML_Template/Blueprint/Widget/WBP_PausedGame.WBP_PausedGame_C|GetWBP_OptionPanel _wbp_pausemenu_2)
            (:Is%20Valid
              (Widget|RemovefromParent (Variables|/Game/HTML_Template/Blueprint/Widget/WBP_PausedGame.WBP_PausedGame_C|GetWBP_OptionPanel _wbp_pausemenu_2)))
            (:Is%20Not%20Valid
              _))
          (Widget|RemovefromParent _wbp_pausemenu_2)
          (Variables|/Script/Engine.PlayerController|SetbShowMouseCursor _returnvalue false)
          (Input|SetInputModeGameOnly _returnvalue))
        (:else)))))

(event Custom|E_LoadLevelInstance
  (params (LevelName :type Name))
  ;[0 0 0] Level Loading/Unloading
  (Game|LoadStreamLevel(byName) LevelName true true))

(event Custom|E_UnloadLevelInstance
  (params (LevelName :type Name))
  ;[0 0 0] Level Loading/Unloading
  (Game|UnloadStreamLevel(byName) LevelName false))

(event Custom|E_MainMenu
  ;[0 0 0] Create Main Menu
  (if (Game|IsGamePaused)
    (Game|SetGamePaused false))
  (bind _returnvalue (UserInterface|CreateWidget "/Game/HTML_Template/Blueprint/Widget/WBP_MainMenu.WBP_MainMenu_C" (Game|GetPlayerController 0)))
  (bind _output_get (Variables|Default|SetWBP_MainMenuRef _returnvalue))
  (UserInterface|Viewport|AddtoViewport _output_get 0)
  (EventDispatchers|BindEventtoPlayGame (Variables|/Game/HTML_Template/Blueprint/Widget/WBP_MainMenu.WBP_MainMenu_C|GetWBP_MainMenuPanel _output_get) (EventDispatchers|CreateEvent :!event Custom|E_StartGame))
  (bind _outactors (Actor|GetAllActorsOfClass "/Game/HTML_Template/Blueprint/Widget/BP_MenuCamera.BP_MenuCamera_C"))
  (Utilities|IsValid (Utilities|Array|Get(acopy) _outactors)
    (:Is%20Valid
      (Game|Player|SetViewTargetwithBlend (Game|GetPlayerController 0) (Utilities|Array|Get(acopy) _outactors) 0.0 "VTBlend_Linear" 0.0 false))))

(event Custom|BE_ResumeGame
  (bind _returnvalue (Game|GetPlayerController 0))
  ;[0 0 0] Create Pause Menu and manage Display On Paused
  (Game|SetGamePaused false)
  (bind _wbp_pausemenu (Variables|Default|GetWBP_PauseMenu)
    (:then
      (Utilities|IsValid (Variables|/Game/HTML_Template/Blueprint/Widget/WBP_PausedGame.WBP_PausedGame_C|GetWBP_OptionPanel _wbp_pausemenu)
        (:Is%20Valid
          (Widget|RemovefromParent (Variables|/Game/HTML_Template/Blueprint/Widget/WBP_PausedGame.WBP_PausedGame_C|GetWBP_OptionPanel _wbp_pausemenu)))
        (:Is%20Not%20Valid
          _))
      (Widget|RemovefromParent _wbp_pausemenu)
      (Variables|/Script/Engine.PlayerController|SetbShowMouseCursor _returnvalue false)
      (Input|SetInputModeGameOnly _returnvalue))
    (:else)))

(event Custom|E_SpawnPlayer
  ;[0 0 0] Spawn player Actor
  (bind _outactors (Actor|GetAllActorsOfClass "/Game/HTML_Template/Blueprint/Character/BP_PlayerStart.BP_PlayerStart_C"))
  (bind _array_element (Utilities|Array|ForEachLoopwithBreak _outactors)
    (:LoopBody
      (if (Utilities|IsValid _array_element)
        (Utilities|FlowControl|Sequence
          (:then_0
            (CallFunction|BreakPlayerStart))
          (:then_1
            (Default|ESpawnPlayerActor _array_element))
          (:then_2
            (bind _outactors_2 (Actor|GetAllActorsOfClass "/Game/HTML_Template/Blueprint/BWflower/BP_bwFlower.BP_bwFlower_C"))
            (Default|EStartMaskTimer _outactors_2)))))))

(event Custom|Break_PlayerStart
  ;[0 0 0] Spawn player Actor
  (Utilities|Array|ForEachLoopwithBreak (stale Custom|E_SpawnPlayer _outactors)) ; enters at Break
)

(event Custom|E_StartGame
  (bind _returnvalue (Game|GetPlayerController 0))
  ;[0 0 0] Start Game
  (Widget|RemovefromParent (Variables|Default|GetWBP_MainMenuRef))
  (Input|SetInputModeGameOnly _returnvalue)
  (Variables|/Script/Engine.PlayerController|SetbShowMouseCursor _returnvalue false)
  ;;[0 0 0] Loading First Level
  (CallFunction|ELoadingScreen (CallFunction|FGetLoadingScreenImage "0"))
  (CallFunction|ELoadStartStreamLevel))

(event Custom|E_LoadingScreen
  (params (LoadingImage :type Texture%202D%20Object%20Reference))
  ;[0 0 0] Create Loading Screen
  (bind _wbp_loadingscreenref (Variables|Default|GetWBP_LoadingScreenRef)
    (:then
      (UserInterface|Viewport|AddtoViewport _wbp_loadingscreenref 100))
    (:else
      (bind _returnvalue (UserInterface|CreateWidget "/Game/HTML_Template/Blueprint/Widget/WBP_LoadingScreen.WBP_LoadingScreen_C" (Game|GetPlayerController 0) LoadingImage))
      (bind _output_get (Variables|Default|SetWBP_LoadingScreenRef _returnvalue))
      (UserInterface|Viewport|AddtoViewport _output_get 100))))

(event Custom|E_LoadStartStreamLevel
  (bind _levelnametoloadatstart (Variables|Default|GetLevelNameToLoadAtStart))
  ;[0 0 0] First Load After Pressing Play
  (if (!= (Utilities|Array|Length _levelnametoloadatstart) 0)
    (for _array_element _levelnametoloadatstart
      (if (Utilities|Name|NotEqual(Name) _array_element "None")
        (Game|LoadStreamLevel(byName) _array_element true true)
        (Utilities|Array|Add (Variables|Default|GetActiveLevels) _array_element))))
  (Utilities|FlowControl|Delay 1.0)
  (CallFunction|ESpawnPlayer)
  (CallFunction|ERemoveLoadingScreen))

(event Custom|E_RemoveLoadingScreen
  ;[0 0 0] Create Loading Screen
  (bind _wbp_loadingscreenref (Variables|Default|GetWBP_LoadingScreenRef)
    (:then
      (Widget|RemovefromParent _wbp_loadingscreenref))
    (:else)))

(event EventBeginPlay
  ;[0 0 0] Initialization
  (CallFunction|EMainMenu))

(fn ConstructionScript)

(fn FGetLoadingScreenImage
  (params (RowName :type Name))
  (bind _returnvalue (Utilities|GetDataTableRow "/Game/HTML_Template/Blueprint/Widget/Data/DT_LoadingScreen.DT_LoadingScreen" RowName)
    (:then
      (return (Utilities|Struct|BreakStruct_LoadingImages _returnvalue)))))