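; BP_Postprocess_Html is a post-process Blueprint that applies a two-color outline material through its PostProcess component.
; The construction script creates a dynamic instance of MI_ColoredOutline and feeds it the two outline color variables and the width.
; RefreshOutline then adds or updates that instance as a full-weight blendable on the component.
; All setup runs at construction, with no active runtime event logic.
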(event EventBeginPlay)

(fn ConstructionScript
  (Utilities|FlowControl|Sequence
    (:then_0
      ;[0 0 0] Create Outline Dynamic Material Intance
      (bind _returnvalue (Rendering|Material|CreateDynamicMaterialInstance "/Game/HTML_Template/Blueprint/PostProcess/Material/MI_ColoredOutline.MI_ColoredOutline" "None" :!class /Script/Engine.KismetMaterialLibrary))
      (Variables|Default|SetDMI_OutlineMaterial _returnvalue))
    (:then_1
      ;[0 0 0] Set Outline Material Parameters
      (Rendering|Material|SetVectorParameterValue (Variables|Default|GetDMI_OutlineMaterial) "OutlineColor1" (Variables|Default|GetOutlineColor1) :!class /Script/Engine.MaterialInstanceDynamic)
      (Rendering|Material|SetVectorParameterValue (Variables|Default|GetDMI_OutlineMaterial) "OutlineColor2" (Variables|Default|GetOutlineColor2) :!class /Script/Engine.MaterialInstanceDynamic)
      (Rendering|Material|SetScalarParameterValue (Variables|Default|GetDMI_OutlineMaterial) "Width" (Variables|Default|GetOutlineWidth) :!class /Script/Engine.MaterialInstanceDynamic))
    (:then_2
      (CallFunction|RefreshOutline))))

(fn RefreshOutline
  ;[0 0 0] Set Post Processing Material
  (Rendering|AddorUpdateBlendable (Variables|Default|GetPostProcess) (Variables|Default|GetDMI_OutlineMaterial) 1.0 :!class /Script/Engine.PostProcessComponent))